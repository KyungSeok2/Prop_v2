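; Test prop character for Propnight: a player-controlled static mesh with movement, camera look and jump.
; Tick offsets the actor without sweep along spring-arm-relative input and rotates the spring arm from axis input.
; Jump applies an upward impulse to the mesh, gated by a ground flag that any mesh hit resets.
; A function swaps mesh and material; torque and survivor-rotation nodes are disconnected.
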(event `InputAxis|MoveRight`
  (params (AxisValue :type "Float (single-precision)"))
  ;[1 1 1] 코멘트
)

(event `InputAxis|MoveForward`
  (params (AxisValue :type "Float (single-precision)"))
  ;[1 1 1] 코멘트
)

(event `self.ReceiveBeginPlay`
  (bind _asbp_survivor_character (cast `/Game/Propnight/GameMode/PlayLevel/BP_SurvivorCharacter` (`GameplayStatics.GetPlayerCharacter` 0))))

(event `InputAction|Jump`
  (params (Key :type "Key Structure"))
  (:`Pressed`
    (if (`self.IsGround`)
      (`PrimitiveComponent.AddImpulseAtLocation` (`self.Static Mesh`) (0.0 0.0 30000.0) (`self.K2_GetActorLocation`) "None")
      (set `self.IsGround` false))))

(event `self.Static Mesh.OnComponentHit`
  (params (HitComponent :type "PrimitiveComponent Object Reference") (OtherActor :type "Actor Object Reference") (OtherComp :type "PrimitiveComponent Object Reference") (NormalImpulse :type "Vector Structure") (Hit :type "HitResult Structure (by ref)"))
  (set `self.IsGround` true))

(event `self.ReceiveTick`
  (params (DeltaSeconds :type "Float (single-precision)"))
  (bind _relativerotation (`SceneComponent.RelativeRotation` (`self.SpringArm`)))
  (`self.K2_AddActorWorldOffset` (* (`KismetMathLibrary.Normal` (+ (* (`KismetMathLibrary.GetForwardVector` _relativerotation) (`self.GetInputAxisValue`)) (* (`KismetMathLibrary.GetRightVector` _relativerotation) (`self.GetInputAxisValue`)))) 5.0))
  (`SceneComponent.K2_AddRelativeRotation` (`self.SpringArm`) (`KismetMathLibrary.MakeRotator` 0.0 (`self.GetInputAxisKeyValue`) (`self.GetInputAxisKeyValue`)) false false))

(fn `BP_PropCharactor_test_AutoGenFunc`
  (params (GetStaticMesh :type "StaticMesh Object Reference") (GetMaterial :type "MaterialInterface Object Reference"))
  (`StaticMeshComponent.SetStaticMesh` (`self.Static Mesh`) GetStaticMesh)
  (`PrimitiveComponent.SetMaterial` (`self.Static Mesh`) 0 GetMaterial))

(fn `UserConstructionScript`)