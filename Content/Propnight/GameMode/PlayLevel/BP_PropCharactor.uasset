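; Player-controlled prop form for a survivor in a prop-hunt mode, with a physics-simulated mesh, impulse jump and per-tick camera-relative movement.
; It stays without collision until SetStaticMesh, bound to the survivor's dispatcher, applies a mesh and enables physics.
; F line-traces from the camera to copy a "prop"-tagged actor's mesh and material; C hides the prop and repossesses the survivor.
; Both actions use request/response event pairs intended for server execution.
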(event `Key|One`
  (params (Key :type "Key Structure"))
  (bind (_returnvalue_roll _returnvalue_pitch _returnvalue_yaw) (`KismetMathLibrary.BreakRotator` (`SceneComponent.K2_GetComponentRotation` (`self.Camera`))))
  (:`Pressed`
    (`SceneComponent.K2_SetWorldRotation` (`self.Static Mesh`) (`KismetMathLibrary.MakeRotator` 0.0 0.0 _returnvalue_yaw) false false)
    (`SceneComponent.K2_SetWorldRotation` (`self.SpringArm`) (`KismetMathLibrary.MakeRotator` 0.0 0.0 _returnvalue_yaw) false false)))

(event `InputAction|Jump`
  (params (Key :type "Key Structure"))
  ;[1 1 1] 점프
  (:`Pressed`
    (if (`self.IsGround`)
      (`PrimitiveComponent.AddImpulseAtLocation` (`self.Static Mesh`) (0.0 0.0 30000.0) (`self.K2_GetActorLocation`) "None")
      (set `self.IsGround` false))))

(event `self.Static Mesh.OnComponentHit`
  (params (HitComponent :type "PrimitiveComponent Object Reference") (OtherActor :type "Actor Object Reference") (OtherComp :type "PrimitiveComponent Object Reference") (NormalImpulse :type "Vector Structure") (Hit :type "HitResult Structure (by ref)"))
  ;[1 1 1] 점프
  (set `self.IsGround` true))

(event `self.ReceiveTick`
  (params (DeltaSeconds :type "Float (single-precision)"))
  (bind _relativerotation (`SceneComponent.RelativeRotation` (`self.SpringArm`)))
  ;[1 1 1] 카메라 정리
  (`self.K2_AddActorWorldOffset` (* (`KismetMathLibrary.Normal` (+ (* (`KismetMathLibrary.GetForwardVector` _relativerotation) (`self.GetInputAxisValue`)) (* (`KismetMathLibrary.GetRightVector` _relativerotation) (`self.GetInputAxisValue`)))) 5.0))
  (`SceneComponent.K2_AddRelativeRotation` (`self.SpringArm`) (`KismetMathLibrary.MakeRotator` 0.0 (`self.GetInputAxisKeyValue`) (`self.GetInputAxisKeyValue`)) false false))

(event `self.ReceiveBeginPlay`
  ;[1 1 1] 생성될때 콜리전 꺼짐
  (`PrimitiveComponent.SetCollisionEnabled` (`self.Static Mesh`) "NoCollision")
  ;[1 1 1] 생성된 내 SurvivorCharacter 부르기
  (bind _asbp_survivor_character (cast `/Game/Propnight/GameMode/PlayLevel/BP_SurvivorCharacter` (`GameplayStatics.GetPlayerCharacter` 0)))
  (bind _output_get (set `self.Survivor Character` _asbp_survivor_character))
  ;[1 1 1] From
  ; SurvivorCharacter
  (add `/Game/Propnight/GameMode/PlayLevel/BP_SurvivorCharacter.EventDispatcher_SetStaticMesh` _output_get (`|CreateDelegate` :!event `Set Static Mesh`)))

(event `req_transform`
  ;[1 0 0] 서버에서 이벤트 실행
  (`self.res_transform`))

(event `Key|F`
  (params (Key :type "Key Structure"))
  ;[1 1 1] 다른 프롭으로 변신
  (:`Pressed`
    (`self.req_transform`)))

(event `res_transform`
  (bind _camera (`self.Camera`))
  (bind _returnvalue (`SceneComponent.K2_GetComponentLocation` _camera))
  (bind _returnvalue_2 (`SceneComponent.GetForwardVector` _camera))
  ;[1 1 1] 카메라 보는 방향으로 라인트레이스 발사
  (bind _outhit (`KismetSystemLibrary.LineTraceSingle` :`Start` (+ _returnvalue (* _returnvalue_2 700)) :`End` (+ _returnvalue (* _returnvalue_2 1200)) :`TraceChannel` "TraceTypeQuery1" :`DrawDebugType` "ForDuration"))
  ;[1 1 1] 대상이 Prop 태그를 가지고 있다면
  (`/Engine/EditorBlueprintResources/StandardMacros.IsValid` (`.HitActor` (`GameplayStatics.BreakHitResult` _outhit))
    (:`Is Valid`
      (if (`self.ActorHasTag` (`.HitActor` (`GameplayStatics.BreakHitResult` _outhit)) "prop")
        ;[1 1 1] 스테틱매시 컴포넌트를 추출
        (for _array_element (`self.K2_GetComponentsByClass` (`.HitActor` (`GameplayStatics.BreakHitResult` _outhit)) "/Script/Engine.StaticMeshComponent")
          (bind _staticmesh (`StaticMeshComponent.StaticMesh` _array_element))
          ;[1 1 1] 스테틱매시, 머터리얼 변경
          (`self.Set Static Mesh` _staticmesh (`StaticMesh.GetMaterial` _staticmesh 0)))))))

(event `res_to_Human`
  (bind _static_mesh (`self.Static Mesh`))
  (bind (_relativerotation_roll _relativerotation_pitch _relativerotation_yaw) (`KismetMathLibrary.BreakRotator` (`SceneComponent.RelativeRotation` (`self.Camera`))))
  ;[1 1 1] 코멘트
  (`SceneComponent.K2_SetRelativeRotation` (`self.Static Mesh`) (`KismetMathLibrary.MakeRotator` 0.0 0.0 _relativerotation_yaw) false false)
  (`SceneComponent.K2_SetRelativeRotation` (`self.SpringArm`) (`KismetMathLibrary.MakeRotator` 0.0 0.0 _relativerotation_yaw) false false)
  (`SceneComponent.SetVisibility` _static_mesh false false)
  (`PrimitiveComponent.SetSimulatePhysics` _static_mesh false)
  (`PrimitiveComponent.SetCollisionEnabled` _static_mesh "NoCollision")
  (`Controller.Possess` (`GameplayStatics.GetPlayerController` 0) (`self.Survivor Character`))
  (`self.EventDispatcher_ViewSurvivorCharacter`))

(event `req_to_Human`
  ;[1 0 0] 서버에서 이벤트 실행
  (`self.res_to_Human`))

(event `Key|C`
  (params (Key :type "Key Structure"))
  ;[1 1 1] 변신 해제
  (:`Pressed`
    (`self.req_to_Human`)))

(event `Key|Q`
  (params (Key :type "Key Structure"))
  (bind _static_mesh (`self.Static Mesh`))
  (bind (_relativerotation_roll _relativerotation_pitch _relativerotation_yaw) (`KismetMathLibrary.BreakRotator` (`SceneComponent.RelativeRotation` _static_mesh)))
  ;[1 1 1] 위치 정렬
  (:`Pressed`
    (`SceneComponent.K2_SetRelativeRotation` _static_mesh (`KismetMathLibrary.MakeRotator` 0.0 0.0 _relativerotation_yaw) false false)))

(fn `Set Static Mesh`
  (params (GetStaticMesh :type "StaticMesh Object Reference") (GetMaterial :type "MaterialInterface Object Reference") (SurvivorCharacter :type "Character Object Reference"))
  (bind _static_mesh (`self.Static Mesh`))
  ;[1 1 1] From
  ; SurvivorCharacter eventdispacher
  ; PropChracter 이벤트그래프 F누를때
  (`StaticMeshComponent.SetStaticMesh` (`self.Static Mesh`) GetStaticMesh)
  (`PrimitiveComponent.SetMaterial` (`self.Static Mesh`) 0 GetMaterial)
  ;[1 1 1] 콜리젼켜진 상태가 아니라면
  ; SurvivorCharacter의 회전 값을 준다
  (if (not (`PrimitiveComponent.K2_IsCollisionEnabled` (`self.Static Mesh`)))
    (`SceneComponent.K2_SetRelativeRotation` (`self.SpringArm`) (`self.K2_GetActorRotation` SurvivorCharacter) false false)
    (`SceneComponent.SetVisibility` _static_mesh true false)
    (`PrimitiveComponent.SetCollisionEnabled` _static_mesh "QueryAndPhysics")
    (`PrimitiveComponent.SetSimulatePhysics` _static_mesh true)
    (`PrimitiveComponent.SetCollisionResponseToChannel` (`self.Static Mesh`) "ECC_Pawn" "ECR_Block")))

(fn `UserConstructionScript`)